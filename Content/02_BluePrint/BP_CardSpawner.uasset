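; BP_CardSpawner plays a list of Niagara effects one after another, apparently a sequence of card visuals.
; Its NextCard event spawns the current list entry at a fixed world location with auto-destroy, then advances the index.
; After a fixed delay the event calls itself until the list ends.
; Nothing in this graph starts the first call.
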(event `NextCard`
  (bind _returnvalue (`NiagaraFunctionLibrary.SpawnSystemAtLocation` (`|GetArrayItem` (`self.NiagaraList`) (`self.NiagaraListIndex`)) (0.0 0.0 210.0) (struct)))
  (bind _output_get (set `self.Niagara` _returnvalue))
  (`NiagaraComponent.SetAutoDestroy` _output_get true)
  (set `self.NiagaraListIndex` (+ (`self.NiagaraListIndex`) 1))
  (`KismetSystemLibrary.Delay` 6.0)
  (if (< (`self.NiagaraListIndex`) (`KismetArrayLibrary.Array_Length` (`self.NiagaraList`)))
    (`self.NextCard`)))

(fn `UserConstructionScript`)