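; BP_Grabbable is a cable-based vine that the player can grab and hang from.
; Three trigger boxes at the cable's start, end and middle particle flag the third-person controller that grabbing is possible and record the touched box.
; GrabVine attaches the character to that box with gravity and movement off, and UngrabVine restores them.
; Tick keeps the middle box on the cable and applies its rotation while grabbed.
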(event `self.TriggerBoxForGrabVine_01.OnComponentBeginOverlap`
  (params (OverlappedComponent :type "PrimitiveComponent Object Reference") (OtherActor :type "Actor Object Reference") (OtherComp :type "PrimitiveComponent Object Reference") (OtherBodyIndex :type Integer) (bFromSweep :type Boolean) (SweepResult :type "HitResult Structure (by ref)"))
  ; Si le joueur entre collision
  (bind _thirdpersoncontroller (`/Game/1_BuePrint/00_GameManagement/BP_FL_Common.GetThirdPersonController`))
  (set `/Game/1_BuePrint/01_Player/BP_ThirdPersonPlayerController.CanGrabVine` true _thirdpersoncontroller)
  (set `/Game/1_BuePrint/01_Player/BP_ThirdPersonPlayerController.BP_Grabbable` self _thirdpersoncontroller)
  (set `self.TriggerBoxCollied` (`self.TriggerBoxForGrabVine_01`)))

(event `self.TriggerBoxForGrabVine_01.OnComponentEndOverlap`
  (params (OverlappedComponent :type "PrimitiveComponent Object Reference") (OtherActor :type "Actor Object Reference") (OtherComp :type "PrimitiveComponent Object Reference") (OtherBodyIndex :type Integer))
  ; Si le joueur sort de la collision
  (bind _thirdpersoncontroller (`/Game/1_BuePrint/00_GameManagement/BP_FL_Common.GetThirdPersonController` :!label _label))
  (set `/Game/1_BuePrint/01_Player/BP_ThirdPersonPlayerController.CanGrabVine` false _thirdpersoncontroller)
  (set `/Game/1_BuePrint/01_Player/BP_ThirdPersonPlayerController.BP_Grabbable` self _thirdpersoncontroller))

(event `self.TriggerBoxForGrabVine_02.OnComponentEndOverlap`
  (params (OverlappedComponent :type "PrimitiveComponent Object Reference") (OtherActor :type "Actor Object Reference") (OtherComp :type "PrimitiveComponent Object Reference") (OtherBodyIndex :type Integer))
  ; Si le joueur sort de la collision
  (goto _label))

(event `self.TriggerBoxForGrabVine_02.OnComponentBeginOverlap`
  (params (OverlappedComponent :type "PrimitiveComponent Object Reference") (OtherActor :type "Actor Object Reference") (OtherComp :type "PrimitiveComponent Object Reference") (OtherBodyIndex :type Integer) (bFromSweep :type Boolean) (SweepResult :type "HitResult Structure (by ref)"))
  ; Si le joueur entre collision
  (bind _thirdpersoncontroller (`/Game/1_BuePrint/00_GameManagement/BP_FL_Common.GetThirdPersonController`))
  (set `/Game/1_BuePrint/01_Player/BP_ThirdPersonPlayerController.CanGrabVine` true _thirdpersoncontroller)
  (set `/Game/1_BuePrint/01_Player/BP_ThirdPersonPlayerController.BP_Grabbable` self _thirdpersoncontroller)
  (set `self.TriggerBoxCollied` (`self.TriggerBoxForGrabVine_02`)))

(event `self.TriggerBoxForGrabVine_03.OnComponentEndOverlap`
  (params (OverlappedComponent :type "PrimitiveComponent Object Reference") (OtherActor :type "Actor Object Reference") (OtherComp :type "PrimitiveComponent Object Reference") (OtherBodyIndex :type Integer))
  ; Si le joueur sort de la collision
  (goto _label))

(event `self.TriggerBoxForGrabVine_03.OnComponentBeginOverlap`
  (params (OverlappedComponent :type "PrimitiveComponent Object Reference") (OtherActor :type "Actor Object Reference") (OtherComp :type "PrimitiveComponent Object Reference") (OtherBodyIndex :type Integer) (bFromSweep :type Boolean) (SweepResult :type "HitResult Structure (by ref)"))
  ; Si le joueur entre collision
  (bind _thirdpersoncontroller (`/Game/1_BuePrint/00_GameManagement/BP_FL_Common.GetThirdPersonController`))
  (set `/Game/1_BuePrint/01_Player/BP_ThirdPersonPlayerController.CanGrabVine` true _thirdpersoncontroller)
  (set `/Game/1_BuePrint/01_Player/BP_ThirdPersonPlayerController.BP_Grabbable` self _thirdpersoncontroller)
  (set `self.TriggerBoxCollied` (`self.TriggerBoxForGrabVine_03`)))

(event `GrabVine`
  (bind _returnvalue (`GameplayStatics.GetPlayerCharacter` 0))
  ; Grab vine
  (`self.K2_AttachToComponent` (`GameplayStatics.GetPlayerCharacter` 0) (`self.TriggerBoxCollied`) "None" "SnapToTarget" "KeepWorld" "KeepWorld" false)
  (`PrimitiveComponent.SetEnableGravity` (`Character.CapsuleComponent` _returnvalue) false)
  (`CharacterMovementComponent.SetMovementMode` (`Character.CharacterMovement` _returnvalue) "MOVE_None" 0)
  (bind _thirdpersoncontroller (`/Game/1_BuePrint/00_GameManagement/BP_FL_Common.GetThirdPersonController`))
  (set `/Game/1_BuePrint/01_Player/BP_ThirdPersonPlayerController.IsVineGrabbed` true _thirdpersoncontroller)
  (`self.K2_SetActorLocation` _returnvalue (`SceneComponent.K2_GetComponentLocation` (`self.TriggerBoxCollied`)) false false))

(event `UngrabVine`
  (bind _returnvalue (`GameplayStatics.GetPlayerCharacter` 0))
  ; UnGrab Vine
  (`self.K2_DetachFromActor` (`GameplayStatics.GetPlayerCharacter` 0) "KeepWorld" "KeepRelative" "KeepRelative")
  (`PrimitiveComponent.SetEnableGravity` (`Character.CapsuleComponent` _returnvalue) true)
  (`CharacterMovementComponent.SetMovementMode` (`Character.CharacterMovement` _returnvalue) "MOVE_Walking" 0)
  (bind _thirdpersoncontroller (`/Game/1_BuePrint/00_GameManagement/BP_FL_Common.GetThirdPersonController`))
  (set `/Game/1_BuePrint/01_Player/BP_ThirdPersonPlayerController.IsVineGrabbed` false _thirdpersoncontroller)
  (`self.K2_SetActorLocation` _returnvalue (`self.K2_GetActorLocation` _returnvalue) true false))

(event `self.ReceiveTick`
  (params (DeltaSeconds :type "Float (single-precision)"))
  (bind _locations (`CableComponent.GetCableParticleLocations` (`self.Cable`)))
  ; Mise a jour de la position de la "TriggerBoxForGrabVine_03"
  (`SceneComponent.K2_SetWorldLocationAndRotation` (`self.TriggerBoxForGrabVine_03`) (`|GetArrayItem` _locations (/ (`KismetArrayLibrary.Array_Length` _locations) 2)) (* (`SceneComponent.K2_GetComponentRotation` (`self.TriggerBoxForGrabVine_02`)) 1.0) false false)
  (bind _thirdpersoncontroller (`/Game/1_BuePrint/00_GameManagement/BP_FL_Common.GetThirdPersonController`))
  (if (`/Game/1_BuePrint/01_Player/BP_ThirdPersonPlayerController.IsVineGrabbed` _thirdpersoncontroller)
    (`self.K2_SetActorRelativeRotation` _thirdpersoncontroller (`SceneComponent.RelativeRotation` (`self.TriggerBoxForGrabVine_03`)) false false)))

(fn `UserConstructionScript`
  (bind _cable (`self.Cable`))
  (`SceneComponent.K2_AttachToComponent` (`self.TriggerBoxForGrabVine_01`) (`self.Cable`) "CableEnd" "KeepRelative" "KeepRelative" "KeepRelative" true)
  (`SceneComponent.K2_AttachToComponent` (`self.TriggerBoxForGrabVine_02`) (`self.Cable`) "CableStart" "KeepRelative" "KeepRelative" "KeepRelative" true)
  (`SceneComponent.K2_SetWorldLocation` (`self.TriggerBoxForGrabVine_03`) (`|GetArrayItem` (`CableComponent.GetCableParticleLocations` _cable) (/ (`KismetArrayLibrary.Array_Length` (`CableComponent.GetCableParticleLocations` _cable)) 2)) false false))