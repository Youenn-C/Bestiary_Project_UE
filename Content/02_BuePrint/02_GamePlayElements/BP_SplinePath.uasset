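; BP_SplinePath is an actor that moves a referenced actor along its spline, serving as a moving platform path.
; A Box overlap enables movement after a one-second delay.
; While enabled, Tick re-attaches the actor to the Scene component every frame and calls MoveObject, which plays a timeline scaled by TimeToCompleteLoop.
; The timeline lerps distance along the spline to set the actor's world location.
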(event `self.Box.OnComponentBeginOverlap`
  (params (OverlappedComponent :type "PrimitiveComponent Object Reference") (OtherActor :type "Actor Object Reference") (OtherComp :type "PrimitiveComponent Object Reference") (OtherBodyIndex :type Integer) (bFromSweep :type Boolean) (SweepResult :type "HitResult Structure (by ref)"))
  (`KismetSystemLibrary.Delay` 1.0)
  (set `self.AttachedActorCanMove` true))

(event `self.ReceiveTick`
  (params (DeltaSeconds :type "Float (single-precision)"))
  ; Platform Movement
  (if (and (`KismetSystemLibrary.IsValid` (`self.AttatchedActor`)) (`self.AttachedActorCanMove`))
    (`self.K2_AttachToComponent` (`self.AttatchedActor`) (`self.Scene`) "None" "KeepRelative" "KeepRelative" "KeepRelative" true)
    (`self.MoveObject`)))

(event `MoveObject`
  (bind _spline (`self.Spline`))
  ; Platform Movement
  (`TimelineComponent.SetPlayRate` (`self.T_Move`) (/ 1.0 (`self.Time to Complete Loop`)))
  (bind (_direction _movetrack) (`Timeline|T_Move`)
    (:`Update`
      (`self.K2_SetActorLocationAndRotation` :`self` (`self.AttatchedActor`) :`NewLocation` (`SplineComponent.GetLocationAtDistanceAlongSpline` _spline (`KismetMathLibrary.Lerp` 0.0 (`SplineComponent.GetSplineLength` _spline) _movetrack) "World")))))

(fn `UserConstructionScript`)