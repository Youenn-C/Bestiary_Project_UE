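; BP_Checkpoint is a checkpoint trigger that records itself as the player's most recent checkpoint.
; When the player pawn begins overlapping its Box, it stores a self reference in LastCheckPoint on the third-person controller.
; It skips the update if it is already the stored checkpoint, and prints a French debug message when the value changes.
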(event `self.Box.OnComponentBeginOverlap`
  (params (OverlappedComponent :type "PrimitiveComponent Object Reference") (OtherActor :type "Actor Object Reference") (OtherComp :type "PrimitiveComponent Object Reference") (OtherBodyIndex :type Integer) (bFromSweep :type Boolean) (SweepResult :type "HitResult Structure (by ref)"))
  (if (== OtherActor (`GameplayStatics.GetPlayerPawn` 0))
    (bind _thirdpersoncontroller (`/Game/1_BuePrint/00_GameManagement/BP_FL_Common.GetThirdPersonController`))
    (if (!= (`/Game/1_BuePrint/01_Player/BP_ThirdPersonPlayerController.LastCheckPoint` _thirdpersoncontroller) self)
      (bind _thirdpersoncontroller_2 (`/Game/1_BuePrint/00_GameManagement/BP_FL_Common.GetThirdPersonController`))
      (set `/Game/1_BuePrint/01_Player/BP_ThirdPersonPlayerController.LastCheckPoint` self _thirdpersoncontroller_2)
      (`KismetSystemLibrary.PrintString` "Checkpoint mis a jour !"))))

(fn `UserConstructionScript`)